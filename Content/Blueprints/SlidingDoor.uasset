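; Sliding door that moves between closed and opened transforms, driven by trigger, toggle or crank events.
; Trigger and Toggle, each gated by an allow flag, play or reverse a duration-scaled timeline, while crank updates set the slide percent directly.
; A shared function lerps the closed mesh toward the opened mesh's transform, adding random shake mid-travel.
; The construction script mirrors the mesh onto both components, using an editor-volume material for the open position when overrides exist.
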(event `self.ReceiveBeginPlay`
  (set `self.Transform When Closed` (`SceneComponent.K2_GetComponentToWorld` (`self.PositionWhenClosed`)) :!label _label)
  (`self.Set Position By Percent` (stale `/Game/Blueprints/Interface/ICrankableObject.CrankWasUpdated` `New Percent Value`) 1.0 :!label _label_2))

(event `/Game/Blueprints/Interface/ICrankableObject.CrankWasUpdated`
  (params (`New Percent Value` :type "Float (single-precision)"))
  (if (`self.dirty`)
    (set `self.dirty` false)
    (goto _label)
    (else
      (goto _label_2))))

(event `/Game/Blueprints/Interface/ITriggerOrToggle.Trigger`
  (bind _slide (`self.Slide`))
  (if (`self.Allow trigger signals`)
    (set `self.Is door open` (not (`self.Is door open`)))
    (`TimelineComponent.SetPlayRate` _slide (/ (`TimelineComponent.GetTimelineLength` _slide) (`self.How long it takes to slide`)) :!label _label_3)
    (if (`self.Is door open`)
      (bind (_direction _percent _shakiness) (`Timeline|Slide` :!label _label_4)
        (:`Update`
          (`self.Set Position By Percent` _percent _shakiness)))
      (else
        (goto _label_4 :!via `Reverse`)))))

(event `/Game/Blueprints/Interface/ITriggerOrToggle.Toggle`
  (params (IsNowOn :type Boolean))
  (if (`self.Allow toggle signals`)
    (set `self.Is door open` IsNowOn)
    (goto _label_3)))

(fn `Set Position By Percent`
  (params (Percent :type "Float (double-precision)") (ShakeMultiplier :type "Float (double-precision)"))
  (bind (_returnvalue_location _returnvalue_rotation _returnvalue_scale) (`KismetMathLibrary.BreakTransform` (`KismetMathLibrary.TLerp` (`self.Transform When Closed`) (`SceneComponent.K2_GetComponentToWorld` (`self.PositionWhenOpened`)) Percent)))
  (`SceneComponent.K2_SetWorldTransform` (`self.PositionWhenClosed`) (`KismetMathLibrary.MakeTransform` (+ _returnvalue_location (select `bool` (and (> Percent 0.0) (< Percent 1.0)) :`true` (* (`KismetMathLibrary.RandomUnitVector`) (* (`self.Shake intensity while sliding`) ShakeMultiplier)))) _returnvalue_rotation _returnvalue_scale) false false))

(fn `UserConstructionScript`
  (`StaticMeshComponent.SetStaticMesh` (`self.PositionWhenClosed`) (`self.Mesh of Door`))
  (`StaticMeshComponent.SetStaticMesh` (`self.PositionWhenOpened`) (`self.Mesh of Door`))
  (for (_array_element _array_index) (`self.Override Materials`)
    (`PrimitiveComponent.SetMaterial` (`self.PositionWhenClosed`) _array_index _array_element)
    (`PrimitiveComponent.SetMaterial` (`self.PositionWhenOpened`) _array_index "/Game/Art/Materials/EditorVolume.EditorVolume")))